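; BP_Button is a menu button that keeps mouse hover and keyboard selection in step and restyles itself to match the input in use.
; Start sets a looping timer that polls CheckFocus every tenth of a second.
; While hovered, the button takes keyboard focus and shows the mouse style; otherwise it shows a key-selected or not-selected style depending on whether it holds keyboard focus.
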(fn Start
  (Utilities|Time|SetTimerbyFunctionName "BP_Button" "CheckFocus" 0.1 true))

(fn CheckFocus
  ;[1 1 1] С помощью чего пользователь хочет нажать на Button
  (if (Widget|IsHovered)
    (Widget|SetKeyboardFocus)
    (Class|Button|SetStyle (Variables|Default|GetMouseStyle))
    (else
      (Class|Button|SetStyle (select (Class|Widget|HasKeyboardFocus) (Variables|Default|GetKeySelected) (Variables|Default|GetKeyNotSelected))))))