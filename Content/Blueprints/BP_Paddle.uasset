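; BP_Paddle is the player-controlled paddle that moves sideways and serves the ball.
; Axis input moves it along Y with a swept, delta-time-scaled offset.
; On BeginPlay it spawns a stationary BP_Ball at its Sphere component, and each axis update snaps the ball's mesh there until launch.
; The StartBall action gives the ball its start speed and sets MoveBall, which stops it following the paddle.
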(event EventBeginPlay
  (CallFunction|CreateBall))

(event Input|ActionEvents|InputActionStartBall
  (params (Key :type Key%20Structure))
  ;[1 1 1] Start Move Ball
  (:Pressed
    (Variables|/Game/Blueprints/BP_Ball.BP_Ball_C|SetSpeed (Variables|Ball|GetBP_Ball) (Variables|Ball|GetStartSpeedBall))
    (Variables|Ball|SetMoveBall true)))

(event Input|AxisEvents|InputAxisMoveHorizont
  (params (AxisValue :type Float%20%28single-precision%29))
  ;[1 1 1] Move Paddle
  (Transformation|AddActorWorldOffset (Math|Vector|MakeVector 0.0 (* AxisValue (Utilities|Time|GetWorldDeltaSeconds) (Variables|Paddle|GetSpeedPaddle)) 0.0) true)
  (CallFunction|MoveHorizontalBall))

(fn ConstructionScript)

(fn CreateBall
  (Variables|Ball|SetMoveBall false)
  (bind _returnvalue (Game|SpawnActorfromClass "/Game/Blueprints/BP_Ball.BP_Ball_C" (Math|Transform|MakeTransform (.location (Transformation|GetWorldTransform (Variables|Default|GetSphere))) "0, 0, 0" "1,1,1") "Undefined" 0 0))
  (bind _output_get (Variables|Ball|SetBP_Ball _returnvalue))
  (bind _asbp_ball (Utilities|Casting|CastToBP_Ball _output_get))
  (Variables|/Game/Blueprints/BP_Ball.BP_Ball_C|SetSpeed _asbp_ball 0.0))

(fn MoveHorizontalBall
  (if (not (Variables|Ball|GetMoveBall))
    (Transformation|SetWorldLocation (Variables|/Game/Blueprints/BP_Ball.BP_Ball_C|GetMesh (Variables|Ball|GetBP_Ball)) (Transformation|GetWorldLocation (Variables|Default|GetSphere)) true false)))