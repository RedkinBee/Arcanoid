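; BP_Block is a grid of blocks that a BP_Ball breaks on contact.
; The construction script adds a static mesh component per cell, spaced by padding over X and Y counts, each with a random material from an array.
; On Hit, it destroys only the struck component when the other actor is a BP_Ball, so one actor holds the whole grid.
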(event EventBeginPlay)

(event Collision|EventHit
  (params (MyComp :type Primitive%20Component%20Object%20Reference) (Other :type Actor%20Object%20Reference) (OtherComp :type Primitive%20Component%20Object%20Reference) (bSelfMoved :type Boolean) (HitLocation :type Vector :default "0, 0, 0") (HitNormal :type Vector :default "0, 0, 0") (NormalImpulse :type Vector :default "0, 0, 0") (Hit :type Hit%20Result%20Structure%20%28by%20ref%29))
  (Utilities|Casting|CastToBP_Ball Other)
  (Components|DestroyComponent MyComp))

(fn ConstructionScript
  (for _index (range 0 (Variables|Default|Getx))
    (for _index_2 (range 0 (Variables|Default|Gety))
      (bind _returnvalue (AddComponent|AddStaticMeshComponent false (Math|Transform|MakeTransform (Math|Vector|MakeVector (* _index (Variables|Default|GetPaddingX)) (* _index_2 (Variables|Default|GetPaddingY)) 0.0))))
      (Rendering|Material|SetMaterial _returnvalue 0 (Utilities|Array|Get(acopy) (Variables|Default|GetMaterial) (Math|Random|RandomIntegerinRange 0 3))))))