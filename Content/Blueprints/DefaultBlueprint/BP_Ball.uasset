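; BP_Ball is a ball actor that travels in a straight line and bounces off what it hits.
; Each tick it makes a swept XY move from Direction and Speed, reflecting Direction about the hit normal on a blocking hit.
; When OnCollisionBall is set, hits on BP_Block skip the reflection.
; Overlapping a KillZVolume destroys the ball.
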(event EventTick
  (params (DeltaSeconds :type Float%20%28single-precision%29))
  ;[1 1 1] Move Ball
  (bind _sweephitresult (Transformation|AddActorWorldOffset (Math|Vector|MakeVector (.x (* (Variables|Default|GetDirection) (* DeltaSeconds (Variables|Default|GetSpeed)))) (.y (* (Variables|Default|GetDirection) (* DeltaSeconds (Variables|Default|GetSpeed)))) 0.0) true))
  (if (.bBlockingHit (Collision|BreakHitResult _sweephitresult))
    (if (not (and (Variables|Default|GetOnCollisionBall) (== (Utilities|GetClass (.HitActor (Collision|BreakHitResult _sweephitresult))) "/Game/Blueprints/DefaultBlueprint/BP_Block.BP_Block_C")))
      (Variables|Default|SetDirection (Math|Vector|GetReflectionVector (Variables|Default|GetDirection) (.Normal (Collision|BreakHitResult _sweephitresult)))))))

(event Collision|EventActorBeginOverlap
  (params (OtherActor :type Actor%20Object%20Reference))
  ;[1 1 1] Destroy
  (Utilities|Casting|CastToKillZVolume OtherActor)
  (Actor|DestroyActor))

(fn ConstructionScript)