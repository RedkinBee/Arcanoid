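; Brick-breaker block field that builds a random layout and handles BP_Ball hits on its blocks.
; The construction script uses a random MultiGate over grid-loop macros to pick one of seven patterns, adding static mesh components and adjusting CountBlock.
; Each block's material encodes its type: normal, two-hit, bonus (spawns a random pickup) or indestructible.
; With OnCollisionBlock off, any hit destroys the block, even indestructible ones, and sets the ball's OnCollisionBall.
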(event EventBeginPlay
  (Variables|UnvisblyVarible|SetMaxBlock (Variables|UnvisblyVarible|GetCountBlock)))

(event Collision|EventHit
  (params (MyComp :type Primitive%20Component%20Object%20Reference) (Other :type Actor%20Object%20Reference) (OtherComp :type Primitive%20Component%20Object%20Reference) (bSelfMoved :type Boolean) (HitLocation :type Vector :default "0, 0, 0") (HitNormal :type Vector :default "0, 0, 0") (NormalImpulse :type Vector :default "0, 0, 0") (Hit :type Hit%20Result%20Structure%20%28by%20ref%29))
  (Variables|Default|SetComponentBlock MyComp)
  (bind _asbp_ball (Utilities|Casting|CastToBP_Ball Other))
  (if (Variables|Default|GetOnCollisionBlock)
    (Variables|/Game/Blueprints/DefaultBlueprint/BP_Ball.BP_Ball_C|SetOnCollisionBall _asbp_ball false)
    ;[1 1 1] ЖИЗНЬ Блока
    ;;[1 1 1] Вторая жизнь
    (if (!= (Rendering|Material|GetMaterial (Variables|Default|GetComponentBlock) 0) (Utilities|Array|Get(acopy) (Variables|UnvisblyVarible|GetMaterial) 1))
      ;;[1 1 1] Не разрушаемый блок
      (if (!= (Rendering|Material|GetMaterial (Variables|Default|GetComponentBlock) 0) (Utilities|Array|Get(acopy) (Variables|UnvisblyVarible|GetMaterial) 3))
        ;;[1 1 1] Бонус
        (if (!= (Rendering|Material|GetMaterial (Variables|Default|GetComponentBlock) 0) (Utilities|Array|Get(acopy) (Variables|UnvisblyVarible|GetMaterial) 2))
          _
          (else
            ;;[1 1 1] Создание рандомного бонуса
            (Game|SpawnActorfromClass (Utilities|Array|Get(acopy) (Variables|UnvisblyVarible|GetClass) (Math|Random|RandomIntegerinRange 0 5)) (Math|Transform|MakeTransform (Transformation|GetWorldLocation (Variables|Default|GetComponentBlock)) "0,45.000000, 0" "0.750000,0.750000,0.750000") "Undefined" 0 0)))
        ;;[1 1 1] В итоге все тлен
        (Components|DestroyComponent (Variables|Default|GetComponentBlock))
        ;;[1 1 1] Подсчет количества блоков
        (Variables|UnvisblyVarible|SetCountBlock (- (Variables|UnvisblyVarible|GetCountBlock) 1)))
      (else
        (Rendering|Material|SetMaterial (Variables|Default|GetComponentBlock) 0 (Utilities|Array|Get(acopy) (Variables|UnvisblyVarible|GetMaterial)))))
    (else
      (Variables|/Game/Blueprints/DefaultBlueprint/BP_Ball.BP_Ball_C|SetOnCollisionBall _asbp_ball true)
      ;[1 1 1] Для бонуса
      ;;[1 1 1] Не разрушаемый блок
      (if (!= (Rendering|Material|GetMaterial (Variables|Default|GetComponentBlock) 0) (Utilities|Array|Get(acopy) (Variables|UnvisblyVarible|GetMaterial) 3))
        ;;[1 1 1] Бонус
        (if (!= (Rendering|Material|GetMaterial (Variables|Default|GetComponentBlock) 0) (Utilities|Array|Get(acopy) (Variables|UnvisblyVarible|GetMaterial) 2))
          _
          (else
            ;;[1 1 1] Создание рандомного бонуса
            (Game|SpawnActorfromClass (Utilities|Array|Get(acopy) (Variables|UnvisblyVarible|GetClass) (Math|Random|RandomIntegerinRange 0 5)) (Math|Transform|MakeTransform (Transformation|GetWorldLocation (Variables|Default|GetComponentBlock)) "0,45.000000, 0" "0.750000,0.750000,0.750000") "Undefined" 0 0)))
        ;;[1 1 1] В итоге все тлен
        (Components|DestroyComponent (Variables|Default|GetComponentBlock))
        ;;[1 1 1] Подсчет количества блоков
        (Variables|UnvisblyVarible|SetCountBlock (- (Variables|UnvisblyVarible|GetCountBlock) 1))
        (else
          ;;[1 1 1] В итоге все тлен
          (Components|DestroyComponent (Variables|Default|GetComponentBlock)))))))

(fn ConstructionScript
  ;[1 1 1] Max количество блоков
  (Variables|UnvisblyVarible|SetCountBlock (* (+ (Variables|RangeBonus|Getx) 1) (+ (Variables|RangeBonus|Gety) 1)))
  ;[1 1 1] Отцентровка блоков
  (Transformation|SetActorLocation (Math|Vector|MakeVector (- (LocalVariables|GetLocationActorY) (Math|Conversions|ToFloat(Integer) (* (- 12 (Variables|RangeBonus|Gety)) 5))) (+ (LocalVariables|GetLocationActorX) (Math|Conversions|ToFloat(Integer) (* (- 12 (Variables|RangeBonus|Getx)) 5))) 0.0) true false)
  (Utilities|FlowControl|MultiGate true false -1
    (:Out%200
      ;[1 1 1] Все идентичны внутри
      (|MassiveBlock
        (:LoopBody
          ;[1 1 1] 1
          ;;[1 1 1] X Paint
          (if (or (== (LocalVariables|GetIndex%20X) (LocalVariables|GetIndex%20Y)) (== (LocalVariables|GetIndex%20X) (- (Variables|RangeBonus|Gety) (LocalVariables|GetIndex%20Y))))
            ;[0.05522 0.02144 1] Create Bonus Block
            (bind _returnvalue (AddComponent|AddStaticMeshComponent false (LocalVariables|GetTransformBlock) :!label _label))
            (Rendering|Material|SetMaterial _returnvalue 0 (Utilities|Array|Get(acopy) (Variables|UnvisblyVarible|GetMaterial) 2))
            (elif (Math|Random|RandomBool)
              ;[0.05332 1 0] Create Random Destroy Block
              (bind _returnvalue_2 (AddComponent|AddStaticMeshComponent false (LocalVariables|GetTransformBlock) :!label _label_2))
              (Rendering|Material|SetMaterial _returnvalue_2 0 (Utilities|Array|Get(acopy) (Variables|UnvisblyVarible|GetMaterial) (Math|Random|RandomIntegerinRange 0 1)))
              (else
                ;;[1 1 1] Подсчет количества блоков
                (Variables|UnvisblyVarible|SetCountBlock (- (Variables|UnvisblyVarible|GetCountBlock) 1))))))))
    (:Out%201
      (|MassiveBlock_2
        (:LoopBody
          ;[1 1 1] 2
          ;;[1 1 1] [  ] Paint
          (if (Math|Boolean|ORBoolean (== (LocalVariables|GetIndex%20X) 0) (== (LocalVariables|GetIndex%20X) (Variables|RangeBonus|Getx)) (== (LocalVariables|GetIndex%20Y) 0) (== (LocalVariables|GetIndex%20Y) (Variables|RangeBonus|Gety)))
            (goto _label)
            (elif (Math|Random|RandomBool)
              ;[1 0 0.9408] Create All Random Block
              (LocalVariables|SetElementMaterials (Math|Random|RandomIntegerinRange 0 3) :!label _label_3)
              (bind _returnvalue_3 (AddComponent|AddStaticMeshComponent false (LocalVariables|GetTransformBlock)))
              (Rendering|Material|SetMaterial _returnvalue_3 0 (Utilities|Array|Get(acopy) (Variables|UnvisblyVarible|GetMaterial) (LocalVariables|GetElementMaterials)))
              (if (== (LocalVariables|GetElementMaterials) 3)
                (Utilities|Array|Add (Variables|Default|GetMeshArray) 0)
                ;;[1 1 1] Подсчет количества блоков
                (Variables|UnvisblyVarible|SetCountBlock (- (Variables|UnvisblyVarible|GetCountBlock) 1)))
              (else
                ;;[1 1 1] Подсчет количества блоков
                (Variables|UnvisblyVarible|SetCountBlock (- (Variables|UnvisblyVarible|GetCountBlock) 1))))))))
    (:Out%202
      (|MassiveBlock_3
        (:LoopBody
          ;[1 1 1] 3
          ;;[1 1 1] Через 1
          (if (== (Math|Integer|%(Integer) (+ (LocalVariables|GetIndex%20X) (LocalVariables|GetIndex%20Y)) 2) 0)
            (goto _label_2)
            (else
              ;;[1 1 1] Подсчет количества блоков
              (Variables|UnvisblyVarible|SetCountBlock (- (Variables|UnvisblyVarible|GetCountBlock) 1)))))))
    (:Out%203
      (|MassiveBlock_4
        (:LoopBody
          ;[1 1 1] столбцы
          (if (not (== (Math|Integer|%(Integer) (LocalVariables|GetIndex%20X) 2) 0))
            ;[1 1 1] Подсчет количества блоков
            (Variables|UnvisblyVarible|SetCountBlock (- (Variables|UnvisblyVarible|GetCountBlock) 1))
            (goto _label_3)))))
    (:Out%204
      (|MassiveBlock_5
        (:LoopBody
          ;[1 1 1] строки
          (if (== (Math|Integer|%(Integer) (LocalVariables|GetIndex%20Y) 2) 0)
            (goto _label_3)
            (else
              ;[1 1 1] Подсчет количества блоков
              (Variables|UnvisblyVarible|SetCountBlock (- (Variables|UnvisblyVarible|GetCountBlock) 1)))))))
    (:Out%205
      (|MassiveBlock_6
        (:LoopBody
          ;[1 1 1] 6
          ;;[1 1 1] +
          (if (or (== (LocalVariables|GetIndex%20Y) 6) (== (LocalVariables|GetIndex%20X) 6))
            (goto _label)
            (elif (Math|Random|RandomBool)
              (goto _label_3)
              (else
                ;;[1 1 1] Подсчет количества блоков
                (Variables|UnvisblyVarible|SetCountBlock (- (Variables|UnvisblyVarible|GetCountBlock) 1))))))))
    (:Out%206
      (|MassiveBlock_6_2
        (:LoopBody
          ;[1 1 1] 7
          ;;[1 1 1] X и + Paint
          (if (Math|Boolean|ORBoolean (== (LocalVariables|GetIndex%20X) (LocalVariables|GetIndex%20Y)) (== (LocalVariables|GetIndex%20X) (- (Variables|RangeBonus|Gety) (LocalVariables|GetIndex%20Y))) (== (LocalVariables|GetIndex%20Y) 6) (== (LocalVariables|GetIndex%20X) 6))
            (goto _label)
            (elif (Math|Random|RandomBool)
              (goto _label_2)
              (else
                ;;[1 1 1] Подсчет количества блоков
                (Variables|UnvisblyVarible|SetCountBlock (- (Variables|UnvisblyVarible|GetCountBlock) 1))))))))))