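; BP_Bonus is a bonus pickup that falls toward the player's paddle to be caught.
; Each tick it moves along negative X at SpeedBonus with sweep and spins by a fixed step per frame.
; Overlapping BP_Paddle increments the NameBonus count in the paddle's BonusMap and destroys the pickup.
; Overlapping a KillZVolume destroys a missed bonus without awarding it.
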(event Collision|EventActorBeginOverlap
  (params (OtherActor :type Actor%20Object%20Reference))
  (Variables|Components|SetOther%20Actor OtherActor)
  (Utilities|FlowControl|Sequence
    (:then_0
      ;[1 1 1] Если словить бонус Paddle'ом
      (bind _asbp_paddle (Utilities|Casting|CastToBP_Paddle (Variables|Components|GetOther%20Actor)))
      (CallFunction|AddBonusMaps _asbp_paddle)
      (Actor|DestroyActor))
    (:then_1
      ;[1 1 1] Если затупить и не словить
      (Utilities|Casting|CastToKillZVolume (Variables|Components|GetOther%20Actor))
      (Actor|DestroyActor))))

(event EventTick
  (params (DeltaSeconds :type Float%20%28single-precision%29))
  ;[1 1 1] Падение бонуса
  (Transformation|AddActorWorldOffset (Math|Vector|MakeVector (* DeltaSeconds (* -1 (Variables|Default|GetSpeedBonus))) 0.0 0.0) true)
  (Class|Actor|AddActorWorldRotation "0,5.000000, 0" true))

(fn ConstructionScript)

(fn AddBonusMaps
  (params (Target :type BP%20Paddle%20Object%20Reference))
  (bind _bonusmap (Variables|/Game/Blueprints/DefaultBlueprint/BP_Paddle.BP_Paddle_C|GetBonusMap Target))
  (Utilities|Map|Add _bonusmap (Variables|Default|GetNameBonus) (+ (.Value (Utilities|Map|Find _bonusmap (Variables|Default|GetNameBonus))) 1)))