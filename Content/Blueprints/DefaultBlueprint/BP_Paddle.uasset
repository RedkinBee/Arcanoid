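; Player paddle pawn for a brick-breaker game that handles movement, ball launch, lives, pause and the HUD.
; Input events spend BonusMap charges on timed speed, size and fire bonuses.
; A looping timer spends charges on extra balls or slow and shrink debuffs.
; MinusBall counts balls and lives, respawning or opening game over, while save and load events persist score, lives and bonuses through BP_SaveScore.
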(event OnComponentBeginOverlap(Sphere)
  (params (OverlappedComponent :type Primitive%20Component%20Object%20Reference) (OtherActor :type Actor%20Object%20Reference) (OtherComp :type Primitive%20Component%20Object%20Reference) (OtherBodyIndex :type Integer) (bFromSweep :type Boolean) (SweepResult :type Hit%20Result%20Structure%20%28by%20ref%29))
  ;[1 1 1] Проверка нарика в месте спавна
  (Utilities|Casting|CastToBP_Ball OtherActor)
  (Variables|StupidBonus|SetBonusBallCreate false))

(event OnComponentEndOverlap(Sphere)
  (params (OverlappedComponent :type Primitive%20Component%20Object%20Reference) (OtherActor :type Actor%20Object%20Reference) (OtherComp :type Primitive%20Component%20Object%20Reference) (OtherBodyIndex :type Integer))
  ;[1 1 1] Проверка нарика в месте спавна
  (Utilities|Casting|CastToBP_Ball OtherActor)
  (Variables|StupidBonus|SetBonusBallCreate true))

(event Custom|BigPaddleANDDEBAFF
  (bind _mesh (Variables|Default|GetMesh))
  (bind _mesh_2 (Variables|Default|GetMesh))
  (bind _returnvalue (Transformation|GetWorldLocation _mesh_2))
  (bind _returnvalue_2 (Transformation|GetWorldLocation _mesh))
  ;[1 1 1] Переработать
  ;;[1 1 1] Большой Paddle
  (if (Math|Boolean|NORBoolean (> (.y _returnvalue_2) 49.0) (< (.y _returnvalue_2) -49.0))
    _
    (elif (> (.y (Transformation|GetWorldLocation (Variables|Default|GetMesh))) 49.0)
      (Transformation|SetWorldLocation _mesh_2 (Math|Vector|MakeVector (.x _returnvalue) 49.0 (.z _returnvalue)) true false)
      (else
        (Transformation|SetWorldLocation _mesh_2 (Math|Vector|MakeVector (.x _returnvalue) -49.0 (.z _returnvalue)) true false))))
  (Transformation|SetWorldScale3D (Variables|Default|GetMesh) "1.000000,1.000000,1.000000")
  (Utilities|Map|Add (Variables|StupidBonus|GetBonusMap) "BigPaddle" (- (.Value (Utilities|Map|Find (Variables|StupidBonus|GetBonusMap) "BigPaddle")) 1))
  (Variables|StupidBonus|SetBonusPaddleBig false)
  (Utilities|FlowControl|Delay (Variables|Paddle|GetTimeBonus))
  (Transformation|SetWorldScale3D (Variables|Default|GetMesh) "1.000000,1.000000,1.000000")
  (Variables|StupidBonus|SetBonusPaddleBig true))

(event Custom|SavePaddle
  (bind _bonusmap (Variables|StupidBonus|GetBonusMap))
  (bind _as_bp_save_score (Variables|Default|GetAs%20BP%20Save%20Score))
  (bind _output_get (Variables|Default|SetAll_Score (Variables|Default|GetScore)))
  (Variables|/Game/Blueprints/Framework/Save/BP_SaveScore.BP_SaveScore_C|SetScore _as_bp_save_score _output_get)
  (Variables|/Game/Blueprints/Framework/Save/BP_SaveScore.BP_SaveScore_C|SetHealthPaddle _as_bp_save_score (Variables|Paddle|GetHealthPaddle))
  (bind _keys (Utilities|Map|Keys _bonusmap))
  (for _array_element _keys
    (Utilities|Map|Add (Variables|/Game/Blueprints/Framework/Save/BP_SaveScore.BP_SaveScore_C|GetBonusMap _as_bp_save_score) _array_element (.Value (Utilities|Map|Find _bonusmap _array_element)))
    (SaveGame|SaveGametoSlot (Variables|Default|GetAs%20BP%20Save%20Score) "score")))

(event Custom|DebaffBonusEvent
  (bind _mesh (Variables|Default|GetMesh))
  (bind _mesh_2 (Variables|Default|GetMesh))
  (bind _returnvalue (Transformation|GetWorldLocation _mesh_2))
  (bind _returnvalue_2 (Transformation|GetWorldLocation _mesh))
  ;[1 1 1] + Шарик
  (if (and (> (.Value (Utilities|Map|Find (Variables|StupidBonus|GetBonusMap) "PlusBall")) 0) (Variables|StupidBonus|GetBonusBallCreate))
    (CallFunction|SpawnBonusBall)
    (Utilities|Map|Add (Variables|StupidBonus|GetBonusMap) "PlusBall" (- (.Value (Utilities|Map|Find (Variables|StupidBonus|GetBonusMap) "PlusBall")) 1))
    (else
      ;[1 1 1] Дебафф скорости
      (if (> (.Value (Utilities|Map|Find (Variables|StupidBonus|GetBonusMap) "LittleSpeedPaddle")) 0)
        (Variables|Paddle|SetSpeedPaddle (/ (Variables|Paddle|GetSpeedPaddle) 2.0))
        (Utilities|Map|Add (Variables|StupidBonus|GetBonusMap) "LittleSpeedPaddle" (- (.Value (Utilities|Map|Find (Variables|StupidBonus|GetBonusMap) "LittleSpeedPaddle")) 1))
        (Variables|Default|SetBonus false)
        (Utilities|FlowControl|Delay (Variables|Paddle|GetTimeBonus))
        (Variables|Paddle|SetSpeedPaddle (* 2 (Variables|Paddle|GetSpeedPaddle)))
        (Variables|Default|SetBonus true)
        (else
          ;[1 1 1] Переработать
          ;;[1 1 1] Дебафф размера
          (if (> (.Value (Utilities|Map|Find (Variables|StupidBonus|GetBonusMap) "MiniPaddle")) 0)
            (Transformation|SetWorldScale3D (Variables|Default|GetMesh) "1.000000,0.500000,1.000000")
            (Variables|StupidBonus|SetDebaff false)
            (Utilities|Map|Add (Variables|StupidBonus|GetBonusMap) "MiniPaddle" (- (.Value (Utilities|Map|Find (Variables|StupidBonus|GetBonusMap) "MiniPaddle")) 1))
            (Variables|Default|SetBonus false)
            (Utilities|FlowControl|Delay (Variables|Paddle|GetTimeBonus))
            (if (Math|Boolean|NORBoolean (> (.y _returnvalue_2) 62.0) (< (.y _returnvalue_2) -62.0))
              _
              (elif (> (.y (Transformation|GetWorldLocation (Variables|Default|GetMesh))) 49.0)
                (Transformation|SetWorldLocation _mesh_2 (Math|Vector|MakeVector (.x _returnvalue) 49.0 (.z _returnvalue)) true false)
                (else
                  (Transformation|SetWorldLocation _mesh_2 (Math|Vector|MakeVector (.x _returnvalue) -49.0 (.z _returnvalue)) true false))))
            (Transformation|SetWorldScale3D (Variables|Default|GetMesh) "1.000000,1.000000,1.000000")
            (Variables|StupidBonus|SetDebaff true)
            (Variables|Default|SetBonus true)))))))

(event Custom|LoadSavePaddle
  (bind _returnvalue (SaveGame|DoesSaveGameExist "score"))
  (if _returnvalue
    (bind _returnvalue_2 (SaveGame|LoadGamefromSlot "score"))
    (bind _asbp_save_score (Utilities|Casting|CastToBP_SaveScore _returnvalue_2))
    (bind _output_get (Variables|Default|SetAs%20BP%20Save%20Score _asbp_save_score))
    (Variables|Default|SetAll_Score (Variables|/Game/Blueprints/Framework/Save/BP_SaveScore.BP_SaveScore_C|GetScore _output_get))
    (Variables|Paddle|SetHealthPaddle (Variables|/Game/Blueprints/Framework/Save/BP_SaveScore.BP_SaveScore_C|GetHealthPaddle _output_get))
    (bind _keys (Utilities|Map|Keys (Variables|/Game/Blueprints/Framework/Save/BP_SaveScore.BP_SaveScore_C|GetBonusMap _output_get)))
    (for _array_element _keys
      (Utilities|Map|Add (Variables|StupidBonus|GetBonusMap) _array_element (.Value (Utilities|Map|Find (Variables|/Game/Blueprints/Framework/Save/BP_SaveScore.BP_SaveScore_C|GetBonusMap _output_get) _array_element))))
    (else
      (bind _returnvalue_3 (SaveGame|CreateSaveGameObject "/Game/Blueprints/Framework/Save/BP_SaveScore.BP_SaveScore_C"))
      (Variables|Default|SetAs%20BP%20Save%20Score _returnvalue_3))))

(event Custom|MinusBall
  (bind _returnvalue (Game|GetPlayerController 0))
  ;[1 1 1] Подсчет жизней и создание шара
  (Variables|StupidBonus|SetBallOnLevel (- (Variables|StupidBonus|GetBallOnLevel) 1))
  (if (<= (Variables|StupidBonus|GetBallOnLevel) 0)
    (if (> (Variables|Paddle|GetHealthPaddle) 0)
      (bind _output_get (Variables|Paddle|SetHealthPaddle (- (stale _output_get) 1)))
      (CallFunction|CreateBall)
      (bind _asbp_game_play_widjet (Utilities|Casting|CastToBP_GamePlayWidjet (Variables|Components|GetWidjetGeneral)))
      (Default|MinusHEALTH _asbp_game_play_widjet)
      (elif (not (Variables|Save|GetIs%20Pause%20Menu%20Opened))
        (bind _returnvalue_2 (UserInterface|CreateWidget "/Game/Blueprints/Framework/Menu/BP_GameOver_faremwork.BP_GameOver_faremwork_C"))
        (UserInterface|Viewport|AddtoViewport _returnvalue_2 0)
        (bind _output_get_2 (Variables|Save|SetIs%20Pause%20Menu%20Opened true))
        (Game|SetGamePaused _output_get_2)
        (Input|SetInputModeGameandUI _returnvalue (Variables|Default|GetPauseMenuWidjet) "DoNotLock" true)
        (Variables|/Script/Engine.PlayerController|SetbShowMouseCursor _returnvalue true)))))

(event EventBeginPlay
  (Utilities|FlowControl|Sequence
    (:then_0
      ;[1 1 1] Автофокус на пешку
      (Input|SetInputModeGameOnly (Game|GetPlayerController 0)))
    (:then_1
      ;[1 1 1] Включить виджет статов
      (bind _returnvalue (UserInterface|CreateWidget "/Game/Blueprints/Framework/GamePlay/BP_GamePlayWidjet.BP_GamePlayWidjet_C" (Game|GetPlayerController 0)))
      (bind _output_get (Variables|Components|SetWidjetGeneral _returnvalue))
      (UserInterface|Viewport|AddtoViewport _output_get 0))
    (:then_2
      (CallFunction|CreateBall))
    (:then_3
      (Utilities|Time|SetTimerbyFunctionName self "DebaffBonusEvent" 15.0 true))))

(event Input|ActionEvents|InputActionStartBall
  (params (Key :type Key%20Structure :default "None"))
  ;[1 1 1] Управление шариком
  ;;[1 1 1] Запуск шарика
  (:Pressed
    (Variables|/Game/Blueprints/DefaultBlueprint/BP_Ball.BP_Ball_C|SetSpeed (Variables|Ball|GetBP_Ball) (Variables|Ball|GetStartSpeedBall))
    (Variables|Ball|SetMoveBall true)))

(event Input|ActionEvents|InputActionEventSpeedPaddle
  (params (Key :type Key%20Structure :default "None"))
  ;[1 1 1] Использование бонуса Скорости
  (:Pressed
    (if (and (Variables|Default|GetBonus) (> (.Value (Utilities|Map|Find (Variables|StupidBonus|GetBonusMap) "SpeedPaddle")) 0))
      (Variables|Paddle|SetSpeedPaddle (* 2 (Variables|Paddle|GetSpeedPaddle)))
      (Utilities|Map|Add (Variables|StupidBonus|GetBonusMap) "SpeedPaddle" (- (.Value (Utilities|Map|Find (Variables|StupidBonus|GetBonusMap) "SpeedPaddle")) 1))
      (Variables|Default|SetBonus false)
      (Utilities|FlowControl|Delay (Variables|Paddle|GetTimeBonus))
      (Variables|Paddle|SetSpeedPaddle (/ (Variables|Paddle|GetSpeedPaddle) 2.0))
      (Variables|Default|SetBonus true))))

(event Input|ActionEvents|InputActionEventFire
  (params (Key :type Key%20Structure :default "None"))
  ;[1 0.6634 0] Шарик убийца (Бонус Fire)
  (:Pressed
    (if (and (Variables|Default|GetBonus) (> (.Value (Utilities|Map|Find (Variables|StupidBonus|GetBonusMap) "Fire")) 0))
      (Variables|/Game/Blueprints/DefaultBlueprint/BP_Block.BP_Block_C|SetOnCollisionBlock (Variables|BlockRef|GetBP_Block_Ref) false)
      (Utilities|Map|Add (Variables|StupidBonus|GetBonusMap) "Fire" (- (.Value (Utilities|Map|Find (Variables|StupidBonus|GetBonusMap) "Fire")) 1))
      (Variables|Default|SetBonus false)
      (Utilities|FlowControl|Delay (Variables|Paddle|GetTimeBonus))
      (Variables|/Game/Blueprints/DefaultBlueprint/BP_Block.BP_Block_C|SetOnCollisionBlock (Variables|BlockRef|GetBP_Block_Ref) true)
      (Variables|Default|SetBonus true))))

(event Input|ActionEvents|InputActionEventBigPaddle
  (params (Key :type Key%20Structure :default "None"))
  (bind _mesh (Variables|Default|GetMesh))
  (bind _mesh_2 (Variables|Default|GetMesh))
  (bind _returnvalue (Transformation|GetWorldLocation _mesh))
  (bind _returnvalue_2 (Transformation|GetWorldLocation _mesh_2))
  ;[1 1 1] Переработать
  ;;[1 1 1] Большой Paddle
  (:Pressed
    (if (and (Variables|StupidBonus|GetBonusPaddleBig) (> (.Value (Utilities|Map|Find (Variables|StupidBonus|GetBonusMap) "BigPaddle")) 0))
      (if (Variables|StupidBonus|GetDebaff)
        (if (Math|Boolean|NORBoolean (> (.y _returnvalue) 49.0) (< (.y _returnvalue) -49.0))
          _
          (elif (> (.y (Transformation|GetWorldLocation (Variables|Default|GetMesh))) 49.0)
            (Transformation|SetWorldLocation _mesh_2 (Math|Vector|MakeVector (.x _returnvalue_2) 49.0 (.z _returnvalue_2)) true false)
            (else
              (Transformation|SetWorldLocation _mesh_2 (Math|Vector|MakeVector (.x _returnvalue_2) -49.0 (.z _returnvalue_2)) true false))))
        (Transformation|SetWorldScale3D (Variables|Default|GetMesh) "1.000000,2.000000,1.000000")
        (Utilities|Map|Add (Variables|StupidBonus|GetBonusMap) "BigPaddle" (- (.Value (Utilities|Map|Find (Variables|StupidBonus|GetBonusMap) "BigPaddle")) 1))
        (Variables|StupidBonus|SetBonusPaddleBig false)
        (Utilities|FlowControl|Delay (Variables|Paddle|GetTimeBonus))
        (Transformation|SetWorldScale3D (Variables|Default|GetMesh) "1.000000,1.000000,1.000000")
        (Variables|StupidBonus|SetBonusPaddleBig true)
        (else
          (CallFunction|BigPaddleANDDEBAFF))))))

(event Input|ActionEvents|InputActionPausePaddle
  (params (Key :type Key%20Structure :default "None"))
  (bind _returnvalue (Game|GetPlayerController 0))
  ;[1 1 1] Пауза
  (:Pressed
    (if (not (Variables|Save|GetIs%20Pause%20Menu%20Opened))
      (bind _returnvalue_2 (UserInterface|CreateWidget "/Game/Blueprints/Framework/Menu/BP_Pause.BP_Pause_C"))
      (bind _asbp_pause (Utilities|Casting|CastToBP_Pause _returnvalue_2))
      (Variables|/Game/Blueprints/Framework/Menu/BP_Pause.BP_Pause_C|SetBP_paddle _asbp_pause self)
      (UserInterface|Viewport|AddtoViewport _returnvalue_2 0)
      (bind _output_get (Variables|Save|SetIs%20Pause%20Menu%20Opened true))
      (Game|SetGamePaused _output_get)
      (Input|SetInputModeGameandUI _returnvalue (Variables|Default|GetPauseMenuWidjet) "DoNotLock" true)
      (Variables|/Script/Engine.PlayerController|SetbShowMouseCursor _returnvalue true))))

(event Input|AxisEvents|InputAxisMoveHorizont
  (params (AxisValue :type Float%20%28single-precision%29))
  ;[1 1 1] Управление шариком
  ;;[1 1 1] Горизонтальное движение шарика
  (Transformation|AddActorWorldOffset (Math|Vector|MakeVector 0.0 (* AxisValue (Utilities|Time|GetWorldDeltaSeconds) (Variables|Paddle|GetSpeedPaddle)) 0.0) true)
  (if (not (Variables|Ball|GetMoveBall))
    (Transformation|SetWorldLocation (Variables|/Game/Blueprints/DefaultBlueprint/BP_Ball.BP_Ball_C|GetMesh (Variables|Ball|GetBP_Ball)) (Transformation|GetWorldLocation (Variables|Default|GetSphere)) true false)))

(fn ConstructionScript)

(fn CreateBall
  (Variables|Ball|SetMoveBall false)
  (bind _returnvalue (Game|SpawnActorfromClass "/Game/Blueprints/DefaultBlueprint/BP_Ball.BP_Ball_C" (Math|Transform|MakeTransform (.location (Transformation|GetWorldTransform (Variables|Default|GetSphere))) "0, 0, 0" "1,1,1") "AdjustIfPossibleButDontSpawnIfColliding" 0 0))
  (bind _output_get (Variables|Ball|SetBP_Ball _returnvalue))
  (bind _asbp_ball (Utilities|Casting|CastToBP_Ball _output_get))
  (Variables|/Game/Blueprints/DefaultBlueprint/BP_Ball.BP_Ball_C|SetSpeed _asbp_ball 0.0)
  (Variables|StupidBonus|SetBallOnLevel 1))

(fn MoveHorizontalBall)

(fn SpawnBonusBall
  (bind _returnvalue (Game|SpawnActorfromClass "/Game/Blueprints/DefaultBlueprint/BP_Ball.BP_Ball_C" (Math|Transform|MakeTransform (.location (Transformation|GetWorldTransform (Variables|Default|GetSphere))) "0, 0, 0" "1,1,1") "AdjustIfPossibleButDontSpawnIfColliding" 0 0))
  (bind _output_get (Variables|Ball|SetBP_Ball _returnvalue))
  (bind _asbp_ball (Utilities|Casting|CastToBP_Ball _output_get))
  (Variables|/Game/Blueprints/DefaultBlueprint/BP_Ball.BP_Ball_C|SetSpeed _asbp_ball (Variables|Ball|GetStartSpeedBall))
  (bind _output_get_2 (Variables|StupidBonus|SetBallOnLevel (+ (stale _output_get_2) 1))))